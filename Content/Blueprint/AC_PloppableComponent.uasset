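; AC_PloppableComponent is an actor component that marks its owner's placement as valid or invalid based on overlaps with other actors.
; It binds to the owner's begin and end overlap events and re-evaluates on BeginPlay and on every change.
; Placement is valid only when nothing overlaps, and the result swaps the first material slot on all the owner's static meshes between ploppable and invalid materials.
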(event `self.ReceiveBeginPlay`
  (bind _returnvalue (`self.GetOwner`))
  (add `Actor.OnActorBeginOverlap` _returnvalue (delegate `OverlapStatusOnChanged`))
  (add `Actor.OnActorEndOverlap` _returnvalue (delegate `OverlapStatusOnChanged`))
  (`self.UpdateState`))

(event `OverlapStatusOnChanged`
  (params (OverlappedActor :type "Actor Object Reference") (OtherActor :type "Actor Object Reference"))
  (`self.UpdateState`))

(fn `UpdateState`
  (bind _output_get (set `self.IsPlacementValid` (== (`KismetArrayLibrary.Array_Length` (`Actor.GetOverlappingActors` (`self.GetOwner`) "/Script/Engine.Actor")) 0)))
  (for _array_element (`Actor.K2_GetComponentsByClass` (`self.GetOwner`) "/Script/Engine.StaticMeshComponent")
    (if _output_get
      (`PrimitiveComponent.SetMaterial` _array_element 0 (`self.PloppableMaterial`))
      (else
        (`PrimitiveComponent.SetMaterial` _array_element 0 (`self.InvalidPloppableMaterial`))))))