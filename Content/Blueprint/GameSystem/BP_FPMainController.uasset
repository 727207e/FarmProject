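; Player controller that runs building placement, with placement mode switched on at BeginPlay.
; Enabling the mode spawns a preview actor far below the world, sets its clickable component to placement mode and adds a ploppable component.
; Each tick, a mouse-cursor line trace moves the preview to the hit point.
; OnBlueprint spawns a building at the preview's transform if the ploppable component reports valid placement.
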(event `self.ReceiveBeginPlay`
  (`self.SetPlacementModeEnable` true))

(event `self.ReceiveTick`
  (params (DeltaSeconds :type "Float (single-precision)"))
  (if (`self.PlacementModeEnable`)
    (`self.UpdatePlacement`)))

(event `self.OnBlueprint`
  (`self.SpawnBuilding`))

(fn `SetPlacementModeEnable`
  (params (IsEnabled :type Boolean))
  (bind _placeableactor (`self.PlaceableActor`))
  (if (== IsEnabled (`self.PlacementModeEnable`))
    (return)
    (else
      (bind _output_get (set `self.PlacementModeEnable` IsEnabled))
      (if _output_get
        (bind _returnvalue (`|SpawnActorFromClass` (`self.PlaceableActorType`) (`KismetMathLibrary.MakeTransform` (0.0 0.0 -10000000.0)) "AlwaysSpawn" "MultiplyWithRoot" null null))
        (bind _output_get_2 (set `self.PlaceableActor` _returnvalue))
        (bind _returnvalue_2 (`self.GetComponentByClass` _output_get_2 "/Game/Blueprint/AC_Clickable.AC_Clickable_C"))
        (`/Engine/EditorBlueprintResources/StandardMacros.IsValid` _returnvalue_2
          (:`Is Valid`
            (`/Game/Blueprint/AC_Clickable.InPlacementMode` _returnvalue_2))
          (:`Is Not Valid`
            _))
        (`AddComponent|NODE_AddAC_PloppableComponent-0` :`self` _output_get_2)
        (else
          (`/Engine/EditorBlueprintResources/StandardMacros.IsValid` _placeableactor
            (:`Is Valid`
              (`self.K2_DestroyActor` _placeableactor))))))))

(fn `SpawnBuilding`
  (bind _returnvalue (`self.GetComponentByClass` (`self.PlaceableActor`) "/Game/Blueprint/AC_PloppableComponent.AC_PloppableComponent_C"))
  (`/Engine/EditorBlueprintResources/StandardMacros.IsValid` _returnvalue
    (:`Is Valid`
      (if (`/Game/Blueprint/AC_PloppableComponent.IsPlacementValid` _returnvalue)
        (`|SpawnActorFromClass` (`self.PlaceableActorType`) (`self.GetTransform` (`self.PlaceableActor`)) "AlwaysSpawn" "MultiplyWithRoot" null null)))))

(fn `UpdatePlacement`
  (bind (_locationx _locationy) (`self.GetMousePosition`))
  (bind (_worldposition _worlddirection) (`GameplayStatics.DeprojectScreenToWorld` self (`KismetMathLibrary.MakeVector2D` _locationx _locationy)))
  (bind _outhit (`KismetSystemLibrary.LineTraceSingle` :`Start` _worldposition :`End` (+ _worldposition (* _worlddirection 100000.0)) :`TraceChannel` "TraceTypeQuery3" :`DrawDebugType` "ForOneFrame"))
  (bind (_bblockinghit _binitialoverlap _time _distance _location) (`GameplayStatics.BreakHitResult` _outhit))
  (if _bblockinghit
    (`self.K2_SetActorLocation` (`self.PlaceableActor`) _location false false)))

(fn `UserConstructionScript`)